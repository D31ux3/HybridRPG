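; Base RPG character Blueprint that can be interacted with to play data-table-driven dialogue.
; Interact, when a dialogue row is set, notifies the instigator, locks interaction, stops the character's movement and sends the line to the RPG game mode's HUD widget.
; ShowNextLine follows each row's NextRow link, restoring the starting row and returning false when the chain ends.
; FinishInteraction clears the interaction lock.
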(event `self.ReceiveBeginPlay`
  (`PrimitiveComponent.SetCastShadow` (`self.DialogueIndicator`) false)
  (bind _asgm_rpg (cast `/Game/Blueprints/GM_RPG` (`GameplayStatics.GetGameMode`)))
  (set `self.GameMode` _asgm_rpg)
  (set `self.ResetRowName` (`self.CurrentRowName`)))

(event `/Game/Blueprints/Interfaces/BPI_Interaction.Interact`
  (params (Instigator :type "/Game/Blueprints/Characters/BP_RPGChar_BASE Object Reference"))
  (if (!= (`self.CurrentRowName`) "None")
    (`self.StartInteraction` Instigator null)
    (`self.StartInteraction` Instigator)
    (`self.ShowDialogueLine`)))

(event `/Game/Blueprints/Interfaces/BPI_Interaction.FinishInteraction`
  (`self.EndInteraction`))

(fn `EndInteraction`
  (set `self.IsInteractionLocked` false))

(fn `ShowDialogueLine`
  (bind _returnvalue (`|GetDataTableRow` "/Game/DataTables/DT_HybridRPG_Dialogue.DT_HybridRPG_Dialogue" (`self.CurrentRowName`))
    (:`then`
      (bind (_dialoguetext _nextrow) (break `/Game/DataTables/S_DialogueData` _returnvalue))
      (`/Game/Widgets/WBP_HUD.ShowDialogue` (`/Game/Blueprints/GM_RPG.HUDWidget` (`self.GameMode`)) self (`self.Name`) _dialoguetext)
      (set `self.Next Row` _nextrow))))

(fn `ShowNextLine`
  (returns (HasNextLine :type Boolean))
  (if (`KismetStringLibrary.IsEmpty` (`self.Next Row`))
    (set `self.CurrentRowName` (`self.ResetRowName`))
    (return false)
    (else
      (set `self.CurrentRowName` (`KismetStringLibrary.Conv_StringToName` (`self.Next Row`)))
      (`self.ShowDialogueLine`)
      (return true))))

(fn `StartInteraction`
  (params (InteractInstigator :type "Actor Object Reference"))
  (set `self.IsInteractionLocked` true)
  (`MovementComponent.StopMovementImmediately` (`self.CharacterMovement`)))

(fn `UserConstructionScript`)